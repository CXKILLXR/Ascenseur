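; BP_Ascenseur is an elevator that moves its Cube component in response to BP_Bouton_Up and BP_Bouton_Down button actors.
; Every tick it looks up both button classes and reads the state of the first instance of each.
; While either button is on, it plays the MonterAscenseur timeline, otherwise it reverses it.
; The timeline's Monter track sets the Cube's relative location, without sweep.
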(event `self.ReceiveTick`
  (params (DeltaSeconds :type "Float (single-precision)"))
  (bind _outactors (`GameplayStatics.GetAllActorsOfClass` "/Game/Ascenseur/BP_Bouton_Up.BP_Bouton_Up_C"))
  (bind _outactors_2 (`GameplayStatics.GetAllActorsOfClass` "/Game/Ascenseur/BP_Bouton_Down.BP_Bouton_Down_C"))
  (if (or (`/Game/Ascenseur/BP_Bouton_Down.BoutonON_Down` (`|GetArrayItem` _outactors_2)) (`/Game/Ascenseur/BP_Bouton_Up.BoutonON_Up` (`|GetArrayItem` _outactors)))
    (bind (_direction _monter) (`Timeline|MonterAscenseur` :!label _label)
      (:`Update`
        (`SceneComponent.K2_SetRelativeLocation` (`self.Cube`) _monter false false)))
    (else
      (goto _label :!via `Reverse`))))

(fn `UserConstructionScript`)